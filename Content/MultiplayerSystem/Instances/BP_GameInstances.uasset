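; Game instance that handles PlayFab accounts, multiplayer lobby creation and the player's chosen character class.
; Init sets the PlayFab title; Login tries username, falls back to email, and, like Register, opens MainMenu on success.
; CreateLobby stores server settings, creates an Advanced Sessions session with name, map, mode and LAN properties, then opens Lobby as a listen server.
; JoinGame only destroys the current session; a failure handler prints PlayFab errors.
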(event Custom|OnFailure_Playfab
  (params (error :type Play%20Fab%20Error%20Structure) (customData :type Object%20Object%20Reference))
  (bind (_haserror _errorcode _errorname _errormessage _errordetails) (Utilities|Struct|BreakPlayFabError error))
  ;[1 1 1] Failure Logic
  (Development|PrintString _errorname)
  (Development|PrintString _errordetails))

(event Custom|OnLoginWithPlayFab_Success
  (params (result :type Client%20Login%20Result%20Structure) (customData :type Object%20Object%20Reference))
  ;[1 1 1] Event Login
)

(event Custom|OnLoginWithEmailAddress_Success
  (params (result :type Client%20Login%20Result%20Structure) (customData :type Object%20Object%20Reference))
  ;[1 1 1] Event Login
)

(event Custom|RegisterSuccesfull_Playfab
  (params (result :type Client%20Register%20Play%20Fab%20User%20Result%20Structure) (customData :type Object%20Object%20Reference))
  ;[1 1 1] Register Logic
)

(event Custom|JoinGame
  ;[1 1 1] Join Game Function
  (|DestroySession (Game|GetPlayerController 0)))

(event Custom|CreateLobby
  (params (ServerName :type String) (ServerMap :type String) (ServerPlayerCount :type Integer) (ServerMode :type String) (ServerMethod_Lan? :type Boolean))
  ;[1 1 1] Advance Session Details
  (Variables|Default|SetServerName ServerName)
  (Variables|Default|SetServerMap ServerMap)
  (Variables|Default|SetServerPlayerCount ServerPlayerCount)
  (Variables|Default|SetServerMode ServerMode)
  (Variables|Default|SetServerMethod_Lan? ServerMethod_Lan?)
  (|AdvancedSession (Utilities|Array|MakeArray (Class|AdvancedSessionsLibrary|MakeLiteralSessionPropertyString "NAME" (Variables|Default|GetServerName)) (Class|AdvancedSessionsLibrary|MakeLiteralSessionPropertyString "MAP" (Variables|Default|GetServerMap)) (Class|AdvancedSessionsLibrary|MakeLiteralSessionPropertyString "MODE" (Variables|Default|GetServerMode)) (Class|AdvancedSessionsLibrary|MakeLiteralSessionPropertyBool "LAN" (Variables|Default|GetServerMethod_Lan?))) (Game|GetPlayerController 0) (Variables|Default|GetServerPlayerCount) 0 (Variables|Default|GetServerMethod_Lan?) true false true true true false false false true false true
    (:OnSuccess
      (Game|OpenLevel(byObjectReference) "/Game/MultiplayerSystem/Maps/Lobby.Lobby" true "listen"))))

(event Custom|SetCharacterClass
  (params (ChossenClass :type Character%20Class%20Reference))
  (Variables|Default|SetChossenCharacterClass ChossenClass))

(event EventLogin
  (params (Username/Email :type String) (Password :type String))
  ;[1 1 1] Event Login
  (|LoginwithPlayFab (Utilities|Struct|MakeClientLoginWithPlayFabRequest 0 0 Password Username/Email) (delegate Custom|OnLoginWithPlayFab_Success) (EventDispatchers|CreateEvent :!event Custom|OnFailure_Playfab)
    (:OnPlayFabResponse
      (if true
        (Game|OpenLevel(byObjectReference) "/Game/MultiplayerSystem/Maps/MainMenu.MainMenu" :!label _label)
        (else
          (|LoginwithEmailAddress (Utilities|Struct|MakeClientLoginWithEmailAddressRequest Username/Email Password) (delegate Custom|OnLoginWithEmailAddress_Success) (EventDispatchers|CreateEvent :!event Custom|OnFailure_Playfab)
            (:OnPlayFabResponse
              (if true
                (goto _label)))))))))

(event EventInit
  ;[1 1 1] PlayFab Settings
  (Class|PlayFabUtilities|SetPlayFabSettings "2C7C4"))

(event EventRegister
  (params (Username :type String) (Email :type String) (Password :type String))
  ;[1 1 1] Register Logic
  (bind _successful (|RegisterPlayFabUser (Utilities|Struct|MakeClientRegisterPlayFabUserRequest Username Email Password Username) (delegate Custom|RegisterSuccesfull_Playfab) (EventDispatchers|CreateEvent :!event Custom|OnFailure_Playfab))
    (:OnPlayFabResponse
      (if _successful
        (Game|OpenLevel(byObjectReference) "/Game/MultiplayerSystem/Maps/MainMenu.MainMenu")))))
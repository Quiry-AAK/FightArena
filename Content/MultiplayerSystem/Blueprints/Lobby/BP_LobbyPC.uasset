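; BP_LobbyPC is the multiplayer lobby player controller, handling each player's lobby UI, name, ready status and character choice.
; Setup creates a host or client widget by authority, enables cursor input and submits the game instance's player name.
; Name, ready toggle (also on R) and character selection pass to BP_LobbyGM, while player-list updates feed the matching widget.
; Match start shows the host UI's loading screen and disables input.
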(event Custom|SelectCharacterOnServer
  (params (Character%20Index :type Integer))
  (Default|SelectCharacterClassbyIndex (Variables|Default|GetLobbyGM_Ref) self Character%20Index)
  (Variables|Default|SetSelectedCharacterIndex Character%20Index))

(event Custom|TryAgainUpdatingLobbyInfo
  (Utilities|FlowControl|Delay 0.1)
  (bind _asbp_lobby_gm (Utilities|Casting|CastToBP_LobbyGM (Game|GetGameMode)))
  (Default|UpdatePlayerLobbyInfo _asbp_lobby_gm self))

(event Custom|OnStartMatch
  (bind _lobbyhostuiref (Variables|Default|GetLobbyHostUIRef)
    (:then
      (Default|ShowLoadingScreen _lobbyhostuiref)
      (Input|DisableInput self (Game|GetPlayerController 0)))
    (:else)))

(event Custom|CreateLobbyUI
  (Networking|SwitchHasAuthority
    (:Authority
      (bind _returnvalue (UserInterface|CreateWidget "/Game/MultiplayerSystem/Widgets/WB_Host.WB_Host_C"))
      (bind _output_get (Variables|Default|SetLobbyWidget _returnvalue))
      (UserInterface|Viewport|AddtoViewport _output_get 0))
    (:Remote
      (bind _returnvalue_2 (UserInterface|CreateWidget "/Game/MultiplayerSystem/Widgets/WB_Client.WB_Client_C"))
      (bind _output_get_2 (Variables|Default|SetLobbyWidget _returnvalue_2))
      (UserInterface|Viewport|AddtoViewport _output_get_2 0))))

(event Custom|SetReadyStatus
  (bind _playerinfo (Variables|Default|GetPlayerInfo))
  (Utilities|Struct|SetmembersinST_PlayerInfo _playerinfo (not (.PlayerIsReady (Utilities|Struct|BreakST_PlayerInfo _playerinfo))))
  (bind _asbp_lobby_gm (Utilities|Casting|CastToBP_LobbyGM (Game|GetGameMode)))
  (Default|UpdatePlayerLobbyInfo _asbp_lobby_gm self))

(event Custom|UpdatePlayerList
  (params (PlayerInfo :type Array%20of%20ST%20Player%20Info%20Structures))
  (bind _output_get (Variables|Default|SetConnectedPlayerInfo PlayerInfo))
  (Networking|SwitchHasAuthority
    (:Authority
      (bind _aswb_host (Utilities|Casting|CastToWB_Host (Variables|Default|GetLobbyWidget)))
      (Default|UpdatePlayerList _aswb_host _output_get))
    (:Remote
      (bind _aswb_client (Utilities|Casting|CastToWB_Client (Variables|Default|GetLobbyWidget)))
      (Default|UpdatePlayerList _aswb_client _output_get))))

(event Custom|SetPlayerNameOnServer
  (params (PlayerName :type Text))
  (Utilities|Struct|SetmembersinST_PlayerInfo (Variables|Default|GetPlayerInfo) PlayerName)
  (bind _asbp_lobby_gm (Utilities|Casting|CastToBP_LobbyGM (Game|GetGameMode)))
  (Default|UpdatePlayerLists _asbp_lobby_gm)
  (Default|UpdatePlayerLobbyInfo _asbp_lobby_gm self))

(event EventBeginPlay
  (CallFunction|SetUp)
  (Variables|Default|SetLobbyGM_Ref (.AsBP%20Lobby%20GM (Utilities|Casting|CastToBP_LobbyGM (Game|GetGameMode)))))

(event Input|KeyboardEvents|R
  (params (Key :type Key%20Structure :default "None"))
  (:Pressed
    (CallFunction|SetReadyStatus)))

(fn ConstructionScript)

(fn SetUp
  (CallFunction|CreateLobbyUI)
  (Variables|Default|SetbShowMouseCursor true)
  (Input|SetInputModeGameandUI self 0 "DoNotLock" false false)
  (CallFunction|SetPlayerNameonServer (Variables|/Game/MultiplayerSystem/Instances/BP_AdvanceGameInstance.BP_AdvanceGameInstance_C|GetPlayerName (.AsBP%20Advance%20Game%20Instance (Utilities|Casting|CastToBP_AdvanceGameInstance (Game|GetGameInstance))))))
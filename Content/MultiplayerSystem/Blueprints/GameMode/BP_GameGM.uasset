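; BP_GameGM is a multiplayer game mode that spawns each player as their selected character and creates the in-game UI.
; HandleStartingNewPlayer restarts each new player at a found player start.
; The pawn class override looks up SelectedCharactersOfAll in BP_AdvanceGameInstance by player name, returning no class if the entry is invalid, without parent fallback.
; BeginPlay chains through server- and client-named events to add a widget for player controller 0 only.
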(event Custom|OnClientInGameUI
  (bind _returnvalue (UserInterface|CreateWidget "/Game/MultiplayerSystem/Widgets/WB_InGameUI.WB_InGameUI_C" (Game|GetPlayerController 0)))
  (UserInterface|Viewport|AddtoViewport _returnvalue 0))

(event Custom|OnServerInGameUI
  (CallFunction|OnClientinGameUI))

(event EventBeginPlay
  (CallFunction|OnServerinGameUI))

(event EventHandleStartingNewPlayer
  (params (NewPlayer :type Player%20Controller%20Object%20Reference))
  (Class|GameModeBase|RestartPlayeratPlayerStart NewPlayer (Class|GameModeBase|FindPlayerStart NewPlayer)))

(fn ConstructionScript)

(fn GetDefaultPawnClassforController
  (params (InController :type Controller%20Object%20Reference))
  (bind _returnvalue (Game|GetGameInstance))
  (bind _playerstate (Variables|/Script/Engine.Controller|GetPlayerState InController))
  (bind _returnvalue_2 (PlayerState|GetPlayerName _playerstate))
  (bind _asbp_advance_game_instance (Utilities|Casting|CastToBP_AdvanceGameInstance _returnvalue))
  (bind _selectedcharactersofall (Variables|/Game/MultiplayerSystem/Instances/BP_AdvanceGameInstance.BP_AdvanceGameInstance_C|GetSelectedCharactersOfAll _asbp_advance_game_instance))
  (bind _value (Utilities|Map|Find _selectedcharactersofall _returnvalue_2))
  (if (Utilities|IsValidClass _value)
    (return _value)
    (else
      (return 0))))
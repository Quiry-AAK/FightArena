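; BP_BaseLobbyGM is the multiplayer lobby game mode that tracks connected players, starts the lobby and kicks players.
; Login and logout update the controller arrays and player info structs, then push the list to every BP_BaseLobbyPC after a short delay.
; UpdatePlayerLists rebuilds that info from the controllers and rebroadcasts it.
; StartLobby server-travels to the Lobby map, then calls OnStartLobbySolo on each lobby controller.
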(event Custom|UpdatePlayerLists
  (Utilities|Array|Clear (Variables|Default|GetCoonectedPlayerInfo))
  (for _array_element (Variables|Default|GetConnectedPlayers)
    (Utilities|Array|Add (Variables|Default|GetCoonectedPlayerInfo) (Variables|/Game/MultiplayerSystem/Blueprints/BaseLobby/BP_BaseLobbyPC.BP_BaseLobbyPC_C|GetPlayerInfo _array_element)))
  (Utilities|FlowControl|Delay 0.2)
  (for _array_element_2 (Variables|Default|GetConnectedPlayers)
    (Default|UpdatePlayerList _array_element_2 (Variables|Default|GetCoonectedPlayerInfo))))

(event Custom|PlayerRemove
  (params (PlayerController :type Player%20Controller%20Object%20Reference))
  (Utilities|Array|RemoveItem (Variables|Default|GetPCs) PlayerController))

(event Custom|PlayerSpawnAdd
  (params (PlayerController :type Player%20Controller%20Object%20Reference))
  (Utilities|Array|Add (Variables|Default|GetPCs) PlayerController))

(event Custom|PlayerControlRemove
  (params (New%20Player :type Player%20Controller%20Object%20Reference))
  (bind _asbp_base_lobby_pc (Utilities|Casting|CastToBP_BaseLobbyPC New%20Player))
  (Utilities|Array|RemoveItem (Variables|Default|GetConnectedPlayers) _asbp_base_lobby_pc)
  (Utilities|Array|RemoveItem (Variables|Default|GetCoonectedPlayerInfo) (Variables|/Game/MultiplayerSystem/Blueprints/BaseLobby/BP_BaseLobbyPC.BP_BaseLobbyPC_C|GetPlayerInfo _asbp_base_lobby_pc))
  (Utilities|FlowControl|Delay 0.2)
  (for _array_element (Variables|Default|GetConnectedPlayers)
    (Default|UpdatePlayerList _array_element (Variables|Default|GetCoonectedPlayerInfo))))

(event Custom|PLayerControlAdd
  (params (New%20Player :type Player%20Controller%20Object%20Reference))
  (bind _asbp_base_lobby_pc (Utilities|Casting|CastToBP_BaseLobbyPC New%20Player))
  (Utilities|Array|Add (Variables|Default|GetConnectedPlayers) _asbp_base_lobby_pc)
  (bind _output_get (Variables|/Game/MultiplayerSystem/Blueprints/BaseLobby/BP_BaseLobbyPC.BP_BaseLobbyPC_C|SetPlayerInfo _asbp_base_lobby_pc (Utilities|Struct|MakeST_PlayerInfo "" false 0 New%20Player)))
  (Utilities|Array|Add (Variables|Default|GetCoonectedPlayerInfo) _output_get)
  (Utilities|FlowControl|Delay 0.2)
  (for _array_element (Variables|Default|GetConnectedPlayers)
    (Default|UpdatePlayerList _array_element (Variables|Default|GetCoonectedPlayerInfo))))

(event EventPostLogin
  (params (NewPlayer :type Player%20Controller%20Object%20Reference))
  (CallFunction|PlayerSpawnAdd NewPlayer)
  (CallFunction|PLayerControlAdd NewPlayer))

(event EventOnLogout
  (params (ExitingController :type Controller%20Object%20Reference))
  (bind _asplayer_controller (Utilities|Casting|CastToPlayerController ExitingController))
  (CallFunction|PlayerRemove _asplayer_controller)
  (CallFunction|PlayerControlRemove _asplayer_controller))

(fn ConstructionScript)

(fn StartLobby
  (Utilities|Casting|CastToBP_AdvanceGameInstance (Game|GetGameInstance))
  (Class|AdvancedSessionsLibrary|ServerTravel "Lobby" false false)
  (for _array_element (Variables|Default|GetPCs)
    (bind _asbp_base_lobby_pc (Utilities|Casting|CastToBP_BaseLobbyPC _array_element))
    (Default|OnStartLobbySolo _asbp_base_lobby_pc)))

(fn KickPC
  (params (PlayerToKick :type Player%20Controller%20Object%20Reference))
  (Class|AdvancedSessionsLibrary|KickPlayer PlayerToKick "test"))
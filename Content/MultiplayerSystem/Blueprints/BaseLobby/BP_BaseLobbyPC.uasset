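; Player controller for the multiplayer base lobby, handling lobby UI, player name and ready status.
; On BeginPlay it sets UI-only input, creates a solo or team, host or client widget from the game instance's team flag and authority, then submits the player name.
; Name and ready changes update PlayerInfo and have BP_BaseLobbyGM refresh player lists.
; UpdatePlayerList passes the received info to the solo widgets only.
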(event Custom|ClientBaseLobbyTeam
  ;[1 1 1] All UI Create Widget Controller
  (bind _returnvalue (UserInterface|CreateWidget "/Game/MultiplayerSystem/Widgets/WB_BaseLobbyTeamClient.WB_BaseLobbyTeamClient_C"))
  (bind _output_get (Variables|Default|SetLobbyWidget _returnvalue))
  (UserInterface|Viewport|AddtoViewport _output_get 0))

(event Custom|ClientBaseLobbySolo
  ;[1 1 1] All UI Create Widget Controller
  (bind _returnvalue (UserInterface|CreateWidget "/Game/MultiplayerSystem/Widgets/WB_BaseLobbySoloClient.WB_BaseLobbySoloClient_C"))
  (bind _output_get (Variables|Default|SetLobbyWidget _returnvalue))
  (UserInterface|Viewport|AddtoViewport _output_get 0))

(event Custom|HostBaseLobbyTeam
  ;[1 1 1] All UI Create Widget Controller
  (bind _returnvalue (UserInterface|CreateWidget "/Game/MultiplayerSystem/Widgets/WB_BaseLobbyTeamHost.WB_BaseLobbyTeamHost_C"))
  (bind _output_get (Variables|Default|SetLobbyWidget _returnvalue))
  (UserInterface|Viewport|AddtoViewport _output_get 0))

(event Custom|OnStartLobbySolo
  ;[1 1 1] Start Button Function
  (Variables|Default|GetBaseLobbySoloUIRef
    (:then
      (Input|DisableInput self (Game|GetPlayerController 0)))
    (:else)))

(event Custom|BaseLobbyUIInputController
  ;[1 1 1] Base Lobby UI Controller
  (Input|SetInputModeUIOnly (Game|GetPlayerController 0) 0 "DoNotLock" false)
  (Variables|Default|SetbShowMouseCursor true))

(event Custom|SetReadyStatus
  (bind _playerinfo (Variables|Default|GetPlayerInfo))
  ;[1 1 1] Player Ready Status Function
  (Utilities|Struct|SetmembersinST_PlayerInfo _playerinfo (not (.PlayerIsReady (Utilities|Struct|BreakST_PlayerInfo _playerinfo))))
  (bind _asbp_base_lobby_gm (Utilities|Casting|CastToBP_BaseLobbyGM (Game|GetGameMode)))
  (Default|UpdatePlayerLists _asbp_base_lobby_gm))

(event Custom|UpdatePlayerList
  (params (PlayerInfo :type Array%20of%20ST%20Player%20Info%20Structures))
  ;[1 1 1] Solo Widgets Update Player List Functions
  (bind _output_get (Variables|Default|SetConnectedPlayerInfo PlayerInfo))
  (Networking|SwitchHasAuthority
    (:Authority
      (bind _aswb_base_lobby_solo_host (Utilities|Casting|CastToWB_BaseLobbySoloHost (Variables|Default|GetLobbyWidget)))
      (Default|UpdatePlayerList _aswb_base_lobby_solo_host _output_get))
    (:Remote
      (bind _aswb_base_lobby_solo_client (Utilities|Casting|CastToWB_BaseLobbySoloClient (Variables|Default|GetLobbyWidget)))
      (Default|UpdatePlayerList _aswb_base_lobby_solo_client _output_get))))

(event Custom|SetPlayerNameOnServer
  (params (PlayerName :type Text))
  ;[1 1 1] Server In Name Function
  (Utilities|Struct|SetmembersinST_PlayerInfo (Variables|Default|GetPlayerInfo) PlayerName)
  (bind _asbp_base_lobby_gm (Utilities|Casting|CastToBP_BaseLobbyGM (Game|GetGameMode)))
  (Default|UpdatePlayerLists _asbp_base_lobby_gm))

(event Custom|HostBaseLobbySolo
  ;[1 1 1] All UI Create Widget Controller
  (bind _returnvalue (UserInterface|CreateWidget "/Game/MultiplayerSystem/Widgets/WB_BaseLobbySoloHost.WB_BaseLobbySoloHost_C"))
  (bind _output_get (Variables|Default|SetLobbyWidget _returnvalue))
  (UserInterface|Viewport|AddtoViewport _output_get 0))

(event EventBeginPlay
  ;[1 1 1] Begin Play
  (CallFunction|BaseLobbyUIInputController)
  (bind _asbp_advance_game_instance (Utilities|Casting|CastToBP_AdvanceGameInstance (Game|GetGameInstance)))
  (if (Variables|/Game/MultiplayerSystem/Instances/BP_AdvanceGameInstance.BP_AdvanceGameInstance_C|GetIsTeam _asbp_advance_game_instance)
    (Networking|SwitchHasAuthority
      (:Authority
        (CallFunction|HostBaseLobbyTeam))
      (:Remote
        (CallFunction|ClientBaseLobbyTeam)))
    (else
      (Networking|SwitchHasAuthority
        (:Authority
          (CallFunction|HostBaseLobbySolo))
        (:Remote
          (CallFunction|ClientBaseLobbySolo)))))
  (CallFunction|SetPlayerNameonServer (Variables|/Game/MultiplayerSystem/Instances/BP_AdvanceGameInstance.BP_AdvanceGameInstance_C|GetPlayerName (.AsBP%20Advance%20Game%20Instance (Utilities|Casting|CastToBP_AdvanceGameInstance (Game|GetGameInstance))))))

(fn ConstructionScript)
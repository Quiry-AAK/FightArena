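; Weapon pickup actor that gives its named weapon to a player's weapon slot and then removes itself.
; The construction script shows the configured weapon mesh on the static mesh component.
; EquipWeapon passes the weapon name, anim blueprint and skeletal mesh to the slot's server equip event.
; It then calls a server destroy event, which relays to a multicast event that destroys the actor.
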(event Custom|OnServerDestroyActor
  (CallFunction|OnMulticastDestroyActor))

(event Custom|OnMulticastDestroyActor
  (Actor|DestroyActor))

(event EventEquipWeapon
  (params (WeaponSlot :type Weapon%20Slot%20Object%20Reference) (AnimBlueprint :type New%20Cyber%20Samurai%20Anim%20Blueprint%20Object%20Reference) (SkeletalMeshComponent :type Skeletal%20Mesh%20Component%20Object%20Reference))
  (Default|OnServerEquipWeapon WeaponSlot (Variables|Default|GetWeaponName) AnimBlueprint SkeletalMeshComponent)
  (CallFunction|OnServerDestroyActor))

(fn ConstructionScript
  (Components|StaticMesh|SetStaticMesh (Variables|Components|GetStaticMesh) (Variables|Default|GetWeaponMesh)))
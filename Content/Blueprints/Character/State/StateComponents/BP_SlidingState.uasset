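; Sliding state component for BP_ThirdPersonCharacter that runs a slope-driven slide.
; Entering blocks move input, zeroes ground friction, applies a forward launch impulse and binds a tick handler to the character.
; Each tick traces the floor and adds slope-scaled forward impulse, or clears the animation's IsSliding flag when slow on flat or uphill ground.
; Exiting restores friction and input, unbinds the tick and starts the character's slide delay.
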(event Custom|SlidingThick
  (params (DeltaTime :type Float%20%28double-precision%29))
  (bind _returnvalue (Components|GetOwner))
  (bind _returnvalue_2 (Transformation|GetActorForwardVector _returnvalue))
  (bind _returnvalue_3 (Transformation|GetActorLocation _returnvalue))
  (bind _asbp_third_person_character (Utilities|Casting|CastToBP_ThirdPersonCharacter _returnvalue))
  (bind _charactermovement (Variables|/Script/Engine.Character|GetCharacterMovement _asbp_third_person_character))
  (bind _returnvalue_4 (Pawn|Components|CharacterMovement|GetLastUpdateVelocity _charactermovement))
  (bind _returnvalue_5 (Math|Vector|VectorLength _returnvalue_4))
  (bind _returnvalue_6 (<= _returnvalue_5 6e+02))
  ;[1 1 1] SlidingThick
  (bind _outhit (Collision|LineTraceByChannel _returnvalue_3 (+ _returnvalue_3 "0.000000,0.000000,-350.000000") "TraceTypeQuery1" false 0 "None"))
  (if (or (and (<= (Math|Vector|DotProduct _returnvalue_2 (* (* (* (* (Variables|Default|GetSlope%20Multiplier) (.OutSlopeRollDegreeAngle (Class|KismetMathLibrary|GetSlopeDegreeAngles _returnvalue_2 (.ImpactNormal (Collision|BreakHitResult _outhit)) (Transformation|GetActorUpVector _returnvalue)))) -1.0) _returnvalue_2) DeltaTime)) 0.0) _returnvalue_6) (and _returnvalue_6 (== (Math|Float|Absolute(Float) (* (* (Variables|Default|GetSlope%20Multiplier) (.OutSlopeRollDegreeAngle (Class|KismetMathLibrary|GetSlopeDegreeAngles _returnvalue_2 (.ImpactNormal (Collision|BreakHitResult _outhit)) (Transformation|GetActorUpVector _returnvalue)))) -1.0)) 0.0)))
    (Variables|/Game/Animation_Blueprints/NewCyberSamuraiAnimBlueprint.NewCyberSamuraiAnimBlueprint_C|SetisSliding (Variables|/Game/Blueprints/Character/BP_ThirdPersonCharacter.BP_ThirdPersonCharacter_C|GetAnimBlueprint _asbp_third_person_character) false)
    (else
      (Physics|AddImpulse (Variables|/Script/Engine.Character|GetCharacterMovement _asbp_third_person_character) (* (* (* (* (Variables|Default|GetSlope%20Multiplier) (.OutSlopeRollDegreeAngle (Class|KismetMathLibrary|GetSlopeDegreeAngles _returnvalue_2 (.ImpactNormal (Collision|BreakHitResult _outhit)) (Transformation|GetActorUpVector _returnvalue)))) -1.0) _returnvalue_2) DeltaTime) true))))

(event EventOnEnter
  (bind _returnvalue (Components|GetOwner))
  (bind _asbp_third_person_character (Utilities|Casting|CastToBP_ThirdPersonCharacter _returnvalue))
  (bind _charactermovement (Variables|/Script/Engine.Character|GetCharacterMovement _asbp_third_person_character))
  ;[1 1 1] SlidingOnEnter
  (Input|SetIgnoreMoveInput (Pawn|GetController _asbp_third_person_character) true)
  (Variables|/Script/Engine.CharacterMovementComponent|SetGroundFriction _charactermovement 0.0)
  (Physics|AddImpulse _charactermovement (* (Transformation|GetActorForwardVector _returnvalue) (Variables|Default|GetSlideFirstForceValue)) true)
  (CallFunction|BindSliding true))

(event EventOnExit
  (bind _returnvalue (Components|GetOwner))
  (bind _asbp_third_person_character (Utilities|Casting|CastToBP_ThirdPersonCharacter _returnvalue))
  ;[1 1 1] SlidingOnExit
  (Default|MakeDelayforSlide _asbp_third_person_character)
  (Variables|/Script/Engine.CharacterMovementComponent|SetGroundFriction (Variables|/Script/Engine.Character|GetCharacterMovement _asbp_third_person_character) 8.0)
  (Input|SetIgnoreMoveInput (Pawn|GetController _asbp_third_person_character) false)
  (CallFunction|BindSliding false))

(fn BindSliding
  (params (Bind :type Boolean))
  (bind _returnvalue (Components|GetOwner))
  (bind _asbp_third_person_character (Utilities|Casting|CastToBP_ThirdPersonCharacter _returnvalue))
  (if Bind
    (EventDispatchers|BindEventtoEPThick _asbp_third_person_character (EventDispatchers|CreateEvent :!event Custom|SlidingThick))
    (else
      (EventDispatchers|UnbindEventfromEPThick _asbp_third_person_character (EventDispatchers|CreateEvent :!event Custom|SlidingThick)))))

(fn GetState
  (return "NewEnumerator4"))
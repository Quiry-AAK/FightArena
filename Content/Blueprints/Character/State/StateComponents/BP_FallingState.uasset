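; BP_FallingState is the falling state component in the character's state system, reporting its own enum value through GetState.
; On enter, it binds an event to the owning BP_ThirdPersonCharacter's move input action and switches on ledge tracing through the character's Ledge member.
; On exit, it unbinds from the move input and switches ledge tracing off, so both are tied to the state's lifetime.
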(event EventOnEnter
  (bind _returnvalue (Components|GetOwner))
  (bind _asbp_third_person_character (Utilities|Casting|CastToBP_ThirdPersonCharacter _returnvalue))
  (EventDispatchers|BindEventtoEPIAMove _asbp_third_person_character (EventDispatchers|CreateEvent _asbp_third_person_character :!event FreeMove))
  (Default|BindTraceLedge (Variables|/Game/MultiplayerSystem/Blueprints/Characters/BP_ThirdPersonCharacter.BP_ThirdPersonCharacter_C|GetLedge _asbp_third_person_character) true))

(event EventOnExit
  (bind _returnvalue (Components|GetOwner))
  (bind _asbp_third_person_character (Utilities|Casting|CastToBP_ThirdPersonCharacter _returnvalue))
  (EventDispatchers|UnbindEventfromEPIAMove _asbp_third_person_character (EventDispatchers|CreateEvent _asbp_third_person_character :!event FreeMove))
  (Default|BindTraceLedge (Variables|/Game/MultiplayerSystem/Blueprints/Characters/BP_ThirdPersonCharacter.BP_ThirdPersonCharacter_C|GetLedge _asbp_third_person_character) false))

(fn GetState
  (return "NewEnumerator2"))
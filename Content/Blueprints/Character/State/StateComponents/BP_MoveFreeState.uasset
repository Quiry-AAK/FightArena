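; BP_MoveFreeState is a character state component, named for free movement, that manages a move event binding.
; OnEnter casts the owner to BP_ThirdPersonCharacter and binds an event to its EPIAMove event, and OnExit unbinds from it.
; GetState identifies the state with a fixed enum value.
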(event EventOnEnter
  (EventDispatchers|BindEventtoEPIAMove (.AsBP%20Third%20Person%20Character (Utilities|Casting|CastToBP_ThirdPersonCharacter (Components|GetOwner))) (EventDispatchers|CreateEvent (.AsBP%20Third%20Person%20Character (Utilities|Casting|CastToBP_ThirdPersonCharacter (Components|GetOwner))) :!event FreeMove)))

(event EventOnExit
  (EventDispatchers|UnbindEventfromEPIAMove (.AsBP%20Third%20Person%20Character (Utilities|Casting|CastToBP_ThirdPersonCharacter (Components|GetOwner))) (EventDispatchers|CreateEvent (.AsBP%20Third%20Person%20Character (Utilities|Casting|CastToBP_ThirdPersonCharacter (Components|GetOwner))) :!event FreeMove)))

(fn GetState
  (return "NewEnumerator0"))
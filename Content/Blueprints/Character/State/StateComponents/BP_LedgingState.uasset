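; BP_LedgingState is the character state component for ledging on BP_ThirdPersonCharacter.
; On enter, it has the owner's Ledge object change walking properties for ledging and play the ledge entry montage.
; On exit, it calls the same walking-property change, also passing true rather than false.
; GetState identifies the state with a fixed enum value.
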(event EventOnEnter
  (bind _returnvalue (Components|GetOwner))
  (bind _asbp_third_person_character (Utilities|Casting|CastToBP_ThirdPersonCharacter _returnvalue))
  (bind _ledge (Variables|/Game/Blueprints/Character/BP_ThirdPersonCharacter.BP_ThirdPersonCharacter_C|GetLedge _asbp_third_person_character))
  (Default|ChangeWalkingPropsforLedging _ledge true)
  (Default|PlayLedgeonEnterMontage _ledge))

(event EventOnExit
  (Default|ChangeWalkingPropsforLedging (Variables|/Game/Blueprints/Character/BP_ThirdPersonCharacter.BP_ThirdPersonCharacter_C|GetLedge (.AsBP%20Third%20Person%20Character (Utilities|Casting|CastToBP_ThirdPersonCharacter (Components|GetOwner)))) true))

(fn GetState
  (return "NewEnumerator3"))
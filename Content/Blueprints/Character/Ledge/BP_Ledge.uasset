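; Ledge-grab component for BP_ThirdPersonCharacter that detects ledges ahead and handles the entry onto them.
; TraceLedge flags a ledge in the AnimBlueprint when a head-height forward trace hits and a higher one misses.
; CalculateBorderLocation steps traces upward to find the last hit, which feeds a Motion Warping target for the entry montage.
; Helpers toggle an event binding on the character and zero velocity and gravity on entry; LedgeMove is empty.
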(event Custom|PlayLedgeOnEnterMontage
  (bind _borderlocation (Variables|Default|GetBorderLocation))
  (bind _character (Variables|Default|GetCharacter))
  (bind (_x _y _z) (Math|Vector|BreakVector _borderlocation))
  ;[1 1 1] LedgeOnEnterMontage
  (Class|MotionWarpingComponent|AddorUpdateWarpTarget (Variables|/Game/Blueprints/Character/BP_ThirdPersonCharacter.BP_ThirdPersonCharacter_C|GetMotionWarp _character) (Utilities|Struct|MakeMotionWarpingTarget "Ledge" (Math|Vector|MakeVector _x _y (- _z (Variables|Default|GetLedgeOffSetZ))) (Math|Conversions|RotationFromXVector (Transformation|GetActorForwardVector (Components|GetOwner))) 0 "None" false))
  (Animation|Montage|PlayMontage (Variables|/Script/Engine.Character|GetMesh _character) "/Game/Animations/CyberSamurai/Basic/Ledge/AM_LedgeEnterNew1.AM_LedgeEnterNew1"))

(event EventBeginPlay
  ;[1 1 1] Construct
  (bind _asbp_third_person_character (Utilities|Casting|CastToBP_ThirdPersonCharacter (Components|GetOwner)))
  (Variables|Default|SetCharacter _asbp_third_person_character))

(fn BindTraceLedge
  (params (Bind :type Boolean))
  (bind _character (Variables|Default|GetCharacter))
  (if Bind
    (EventDispatchers|BindEventtoEPThick _character (EventDispatchers|CreateEvent :!event TraceLedge))
    (else
      (EventDispatchers|UnbindEventfromEPThick _character (EventDispatchers|CreateEvent :!event TraceLedge)))))

(fn TraceLedge
  (params (Delta%20Seconds :type Float%20%28double-precision%29))
  (bind _returnvalue (Math|Float|MakeLiteralFloat 3e+01))
  (bind _character (Variables|Default|GetCharacter))
  (bind _returnvalue_2 (Transformation|GetActorForwardVector _character))
  (bind _mesh (Variables|/Script/Engine.Character|GetMesh _character))
  (bind _returnvalue_3 (Transformation|GetBoneTransform _mesh "Head" "RTS_World"))
  (bind _location (Math|Transform|BreakTransform _returnvalue_3))
  (bind (_x _y _z) (Math|Vector|BreakVector _location))
  (bind _returnvalue_4 (+ _z _returnvalue))
  (bind _returnvalue_5 (Math|Vector|MakeVector _x _y _returnvalue_4))
  (bind (_outhit _returnvalue_6) (Collision|LineTraceByChannel _location (+ _location (* _returnvalue_2 (Variables|Default|GetLedge%20Distance))) "TraceTypeQuery1" false 0 "None"))
  (bind _returnvalue_7 (Collision|LineTraceByChannel _returnvalue_5 (+ _returnvalue_5 (* _returnvalue_2 (Math|Float|MakeLiteralFloat 1e+02))) "TraceTypeQuery1" false 0 "None"))
  (if (and _returnvalue_6 (not _returnvalue_7))
    (CallFunction|CalculateBorderLocation)
    (Variables|/Game/Animation_Blueprints/NewCyberSamuraiAnimBlueprint.NewCyberSamuraiAnimBlueprint_C|SetIsLedging (Variables|/Game/Blueprints/Character/BP_ThirdPersonCharacter.BP_ThirdPersonCharacter_C|GetAnimBlueprint (Variables|Default|GetCharacter)) true)))

(fn ChangeWalkingPropsforLedging
  (params (Enter :type Boolean))
  (bind _character (Variables|Default|GetCharacter))
  (bind _charactermovement (Variables|/Script/Engine.Character|GetCharacterMovement _character))
  (if Enter
    (Variables|/Script/Engine.MovementComponent|SetVelocity _charactermovement "0, 0, 0")
    (Variables|/Script/Engine.CharacterMovementComponent|SetGravityScale _charactermovement 0.0)))

(fn LedgeMove)

(fn CalculateBorderLocation
  (bind _character (Variables|Default|GetCharacter))
  (bind _ledge_distance (Variables|Default|GetLedge%20Distance))
  (bind _returnvalue (Transformation|GetActorForwardVector _character))
  (bind _mesh (Variables|/Script/Engine.Character|GetMesh _character))
  (bind _returnvalue_2 (Transformation|GetBoneTransform _mesh "Head" "RTS_World"))
  (bind _returnvalue_3 (* _returnvalue _ledge_distance))
  (bind _location (Math|Transform|BreakTransform _returnvalue_2))
  (bind (_x _y _z) (Math|Vector|BreakVector _location))
  (bind _returnvalue_4 (+ _location _returnvalue_3))
  (bind (_x_2 _y_2 _z_2) (Math|Vector|BreakVector _returnvalue_4))
  (bind _index (Utilities|FlowControl|ForLoopwithBreak 0 10 :!label _label)
    (:LoopBody
      (bind (_outhit _returnvalue_5) (Collision|LineTraceByChannel (Math|Vector|MakeVector _x _y (+ _z (* _index (Math|Float|MakeLiteralFloat 5.0)))) (Math|Vector|MakeVector _x_2 _y_2 (+ (* _index (Math|Float|MakeLiteralFloat 5.0)) _z_2)) "TraceTypeQuery1" false 0 "ForDuration"))
      (if _returnvalue_5
        (Variables|Default|SetBorderLocation (.Location (Collision|BreakHitResult _outhit)))
        (else
          (goto _label Break))))))
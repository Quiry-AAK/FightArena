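; Ledge-grab component for BP_ThirdPersonCharacter that detects a ledge ahead and plays the grab entry animation.
; CheckLedge traces forward from head height and just above it, accepting a low hit with a clear upper trace.
; A hit flags the AnimBP, unbinds from the character's EPThick dispatcher and motion-warps the entry montage to the hit point.
; A separate helper zeroes velocity and gravity for ledging but is not called here; LedgeMove is an empty stub.
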(event Custom|PlayLedgeOnEnterMontage
  (bind _character (Variables|Default|GetCharacter))
  ;[1 1 1] LedgeOnEnterMontage
  (Class|MotionWarpingComponent|AddorUpdateWarpTarget (Variables|/Game/Blueprints/Character/BP_ThirdPersonCharacter.BP_ThirdPersonCharacter_C|GetMW_Ledge _character) (Utilities|Struct|MakeMotionWarpingTarget "Ledge" (Variables|Default|GetBorderLocation) "0.000000,0.000000,0.000000" 0 "None" false))
  (Animation|Montage|PlayMontage (Variables|/Script/Engine.Character|GetMesh _character) "/Game/Animations/CyberSamurai/Basic/Ledge/AM_LedgeEnter.AM_LedgeEnter"))

(event EventBeginPlay
  ;[1 1 1] Construct
  (bind _asbp_third_person_character (Utilities|Casting|CastToBP_ThirdPersonCharacter (Components|GetOwner)))
  (Variables|Default|SetCharacter _asbp_third_person_character))

(fn BindLedge
  (params (Bind :type Boolean))
  (bind _character (Variables|Default|GetCharacter))
  (if Bind
    (EventDispatchers|BindEventtoEPThick _character (EventDispatchers|CreateEvent :!event CheckLedge))
    (else
      (EventDispatchers|UnbindEventfromEPThick _character (EventDispatchers|CreateEvent :!event CheckLedge)))))

(fn CheckLedge
  (params (Delta%20Seconds :type Float%20%28double-precision%29))
  (bind _returnvalue (Math|Float|MakeLiteralFloat 3e+01))
  (bind _character (Variables|Default|GetCharacter))
  (bind _returnvalue_2 (Transformation|GetActorForwardVector _character))
  (bind _mesh (Variables|/Script/Engine.Character|GetMesh _character))
  (bind _returnvalue_3 (Transformation|GetBoneTransform _mesh "Head" "RTS_World"))
  (bind _location (Math|Transform|BreakTransform _returnvalue_3))
  (bind (_x _y _z) (Math|Vector|BreakVector _location))
  (bind _returnvalue_4 (+ _z _returnvalue))
  (bind _returnvalue_5 (Math|Vector|MakeVector _x _y _returnvalue_4))
  (bind (_outhit _returnvalue_6) (Collision|LineTraceByChannel _location (+ _location (* _returnvalue_2 (Variables|Default|GetLedge%20Distance))) "TraceTypeQuery1" false 0 "ForDuration"))
  (bind _returnvalue_7 (Collision|LineTraceByChannel _returnvalue_5 (+ _returnvalue_5 (* _returnvalue_2 (Math|Float|MakeLiteralFloat 1e+02))) "TraceTypeQuery1" false 0 "ForDuration"))
  (if (and _returnvalue_6 (not _returnvalue_7))
    (Variables|Default|SetBorderLocation (.Location (Collision|BreakHitResult _outhit)))
    (Variables|/Game/Animation_Blueprints/NewCyberSamuraiAnimBlueprint.NewCyberSamuraiAnimBlueprint_C|SetIsLedging (Variables|/Game/Blueprints/Character/BP_ThirdPersonCharacter.BP_ThirdPersonCharacter_C|GetAnimBlueprint (Variables|Default|GetCharacter)) true)
    (CallFunction|BindLedge false)
    (CallFunction|PlayLedgeonEnterMontage)))

(fn ChangeWalkingPropsforLedging
  (params (Enter :type Boolean))
  (bind _character (Variables|Default|GetCharacter))
  (bind _charactermovement (Variables|/Script/Engine.Character|GetCharacterMovement _character))
  (if Enter
    (Variables|/Script/Engine.MovementComponent|SetVelocity _charactermovement "0, 0, 0")
    (Variables|/Script/Engine.CharacterMovementComponent|SetGravityScale _charactermovement 0.0)
    (CallFunction|PlayLedgeonEnterMontage)))

(fn LedgeMove)